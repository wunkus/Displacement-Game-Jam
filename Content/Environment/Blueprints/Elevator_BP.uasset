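; Elevator actor whose two sliding doors open after a short delay at game start and close when something steps into its volume.
; A single timeline lerps both doors apart along relative X from their cached start positions and plays in reverse to close them.
; Closing triggers once, on the first capsule component overlap, and both opening and closing play 2D sounds.
; The file contains no cabin movement.
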(event OnComponentBeginOverlap(ElevatorVolume)
  (params (OverlappedComponent :type Primitive%20Component%20Object%20Reference) (OtherActor :type Actor%20Object%20Reference) (OtherComp :type Primitive%20Component%20Object%20Reference) (OtherBodyIndex :type Integer) (bFromSweep :type Boolean) (SweepResult :type Hit%20Result%20Structure%20%28by%20ref%29))
  (Utilities|Casting|CastToCapsuleComponent OtherComp)
  (Utilities|FlowControl|DoOnce false
    (:Completed
      (Audio|SpawnSound2D "/Game/Environment/SFX/DoorClosing.DoorClosing" 1.0 1.0 1.0 0)
      (bind _alpha (Timeline|ElevatorDoorAnimation Reverse)
        (:Update
          (Transformation|SetRelativeLocation (Variables|Default|GetElevatorDoor) (Math|Vector|Lerp(Vector) (Variables|Default|GetDoor1StartLocation) (Math|Vector|MakeVector (- (.x (Variables|Default|GetDoor1StartLocation)) 126.0) 0.0 0.0) _alpha) false false)
          (Transformation|SetRelativeLocation (Variables|Default|GetElevatorDoor1) (Math|Vector|Lerp(Vector) (Variables|Default|GetDoor2StartLocation) (Math|Vector|MakeVector (+ (.x (Variables|Default|GetDoor2StartLocation)) 126.0) 0.0 0.0) _alpha) false false))))))

(event Custom|OpenElevator
  (Audio|SpawnSound2D "/Game/Environment/SFX/DoorOpen.DoorOpen" 1.0 1.0 1.0 0)
  (bind _alpha (Timeline|ElevatorDoorAnimation Play)
    (:Update
      (Transformation|SetRelativeLocation (Variables|Default|GetElevatorDoor) (Math|Vector|Lerp(Vector) (Variables|Default|GetDoor1StartLocation) (Math|Vector|MakeVector (- (.x (Variables|Default|GetDoor1StartLocation)) 126.0) 0.0 0.0) _alpha) false false)
      (Transformation|SetRelativeLocation (Variables|Default|GetElevatorDoor1) (Math|Vector|Lerp(Vector) (Variables|Default|GetDoor2StartLocation) (Math|Vector|MakeVector (+ (.x (Variables|Default|GetDoor2StartLocation)) 126.0) 0.0 0.0) _alpha) false false))))

(event EventBeginPlay
  (Variables|Default|SetDoor1StartLocation (Variables|/Script/Engine.SceneComponent|GetRelativeLocation (Variables|Default|GetElevatorDoor)))
  (Variables|Default|SetDoor2StartLocation (Variables|/Script/Engine.SceneComponent|GetRelativeLocation (Variables|Default|GetElevatorDoor1)))
  (Utilities|FlowControl|Delay 5.0)
  (CallFunction|OpenElevator))

(fn ConstructionScript)