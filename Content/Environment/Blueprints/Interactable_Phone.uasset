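; Interactable phone prop that plays a dial sound when the player interacts with it.
; On BeginPlay it binds to the first-person character's hover, unhover and interact events, ignoring any that target other actors.
; Hovering shows an icon and arms interaction, and unhovering hides it again.
; Each interaction plays the dial as a 2D sound with a slightly randomized pitch.
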(event Custom|Hovered
  (params (HitActor :type Actor%20Object%20Reference))
  (if (== HitActor self)
    (Development|SetHiddeninGame (Variables|Default|GetIcon) false false)
    (Variables|Default|SetIsHovered true)))

(event Custom|UnHovered
  (params (HitActor :type Actor%20Object%20Reference))
  (if (== HitActor self)
    (Development|SetHiddeninGame (Variables|Default|GetIcon) true false)
    (Variables|Default|SetIsHovered false)))

(event Custom|Interacted
  (params (HitActor :type Actor%20Object%20Reference))
  (if (== HitActor self)
    (if (Variables|Default|GetIsHovered)
      (Audio|PlaySound2D "/Game/Environment/SFX/PhoneDial.PhoneDial" 1.0 (Math|Random|RandomFloatinRange 0.8 1.2) 0.0 0 0))))

(event EventBeginPlay
  (bind _asbp_first_person_character (Utilities|Casting|CastToBP_FirstPersonCharacter (Game|GetPlayerCharacter 0)))
  (EventDispatchers|BindEventtoInteractHover _asbp_first_person_character (delegate Custom|Hovered))
  (EventDispatchers|BindEventtoInteractUnhover _asbp_first_person_character (delegate Custom|UnHovered))
  (EventDispatchers|BindEventtoInteract _asbp_first_person_character (delegate Custom|Interacted)))

(fn ConstructionScript)