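; Elevator counter actor that displays a text value, such as a floor readout, on a widget component.
; Both the construction script and BeginPlay cast the component's widget to ElevatorCounter and set its ElevatorCounterText from the actor's Text variable.
; Setting it in both places applies the text at construction as well as at runtime.
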(event EventBeginPlay
  (bind _aselevator_counter (Utilities|Casting|CastToElevatorCounter (UserInterface|GetWidget (Variables|Default|GetWidget))))
  (Variables|/Script/UMG.TextBlock|SetText (Variables|/Game/Environment/Widgets/ElevatorCounter.ElevatorCounter_C|GetElevatorCounterText _aselevator_counter) (Variables|Default|GetText)))

(event Collision|EventActorBeginOverlap
  (params (OtherActor :type Actor%20Object%20Reference)))

(event EventTick
  (params (DeltaSeconds :type Float%20%28single-precision%29)))

(fn ConstructionScript
  (bind _aselevator_counter (Utilities|Casting|CastToElevatorCounter (UserInterface|GetWidget (Variables|Default|GetWidget))))
  (Variables|/Script/UMG.TextBlock|SetText (Variables|/Game/Environment/Widgets/ElevatorCounter.ElevatorCounter_C|GetElevatorCounterText _aselevator_counter) (Variables|Default|GetText)))