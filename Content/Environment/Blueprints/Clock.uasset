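; Clock is an environment Blueprint that shows the real current time on hour and minute hands.
; On BeginPlay it sets the hands, then a looping one-second timer updates them.
; Each update reads Now and sets the pitch of HourArm and MinuteArm from the hour over 12 and the minute over 60 of a full negative turn.
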(event Custom|ChooseHandPosition
  (bind _returnvalue (Math|DateTime|Now))
  (Transformation|SetRelativeRotation (Variables|Default|GetHourArm) (Math|Rotator|MakeRotator 0.0 (* (/ (.hour _returnvalue) 12) -3.6e+02) 0.0) false false)
  (Transformation|SetRelativeRotation (Variables|Default|GetMinuteArm) (Math|Rotator|MakeRotator 0.0 (* (/ (.minute _returnvalue) 60) -3.6e+02) 0.0) false false))

(event EventBeginPlay
  (CallFunction|ChooseHandPosition)
  (Utilities|Time|SetTimerbyEvent (delegate Custom|ChooseHandPosition) 1.0 true))

(fn ConstructionScript)