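; An interactable elevator button that takes the player to another level when pressed.
; It binds to the first-person character's hover, unhover and interact events, showing an icon while hovered.
; On a one-time press it plays sounds, clears its tags and outline stencil, closes the nearest Elevator_BP and freezes player movement.
; After a short delay it opens the assigned level.
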(event Custom|Hovered
  (params (HitActor :type Actor%20Object%20Reference))
  (if (== HitActor self)
    (Development|SetHiddeninGame (Variables|Default|GetIcon) false false)
    (Variables|Default|SetIsHovered true)))

(event Custom|UnHovered
  (params (HitActor :type Actor%20Object%20Reference))
  (if (== HitActor self)
    (Development|SetHiddeninGame (Variables|Default|GetIcon) true false)
    (Variables|Default|SetIsHovered false)))

(event Custom|Interacted
  (params (HitActor :type Actor%20Object%20Reference))
  (if (== HitActor self)
    (if (Variables|Default|GetIsHovered)
      (if (Variables|Default|GetIsInteractable)
        (Utilities|FlowControl|Sequence
          (:then_0
            (Audio|PlaySound2D "/Game/Environment/SFX/button-press-beep-269718.button-press-beep-269718" 1.0 1.0 0.1 0 0)
            (Audio|PlaySound2D "/Game/Environment/SFX/ElevatorAmbience.ElevatorAmbience" 3.0 1.0 0.0 0 0)
            (Utilities|Array|Clear (Variables|Actor|GetTags))
            (Rendering|SetCustomDepthStencilValue (Variables|Default|GetInteractableObject) 0)
            (Development|SetHiddeninGame (Variables|Default|GetIcon) true false)
            (Variables|Default|SetIsInteractable false))
          (:then_1
            (bind _outactors (Actor|GetAllActorsOfClass "/Game/Environment/Blueprints/Elevator_BP.Elevator_BP_C"))
            (bind _aselevator_bp (Utilities|Casting|CastToElevator_BP (.ReturnValue (Actor|FindNearestActor (Transformation|GetActorLocation) _outactors))))
            (Default|CloseElevator _aselevator_bp)
            (bind _asbp_first_person_character (Utilities|Casting|CastToBP_FirstPersonCharacter (Game|GetPlayerCharacter 0)))
            (Pawn|Components|CharacterMovement|DisableMovement (Variables|/Script/Engine.Character|GetCharacterMovement _asbp_first_person_character))
            (Utilities|FlowControl|Delay 5.0)
            (Game|OpenLevel(byObjectReference) (Variables|Default|GetLevel))))))))

(event EventBeginPlay
  (bind _asbp_first_person_character (Utilities|Casting|CastToBP_FirstPersonCharacter (Game|GetPlayerCharacter 0)))
  (EventDispatchers|BindEventtoInteractHover _asbp_first_person_character (delegate Custom|Hovered))
  (EventDispatchers|BindEventtoInteractUnhover _asbp_first_person_character (delegate Custom|UnHovered))
  (EventDispatchers|BindEventtoInteract _asbp_first_person_character (delegate Custom|Interacted)))

(fn ConstructionScript)