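; Trigger actor that plays a one-shot scripted lighting sequence when the first-person character enters its sphere.
; The overlap disables the sphere, then switches on six hanging spotlights one by one with timed delays, each via TurnOnLight setting intensity, emissive material parameter and a positional sound.
; Afterwards it hides the spotlight group with a buzz sound, then lights a final glove spotlight and its fixture.
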(event OnComponentBeginOverlap(Sphere)
  (params (OverlappedComponent :type Primitive%20Component%20Object%20Reference) (OtherActor :type Actor%20Object%20Reference) (OtherComp :type Primitive%20Component%20Object%20Reference) (OtherBodyIndex :type Integer) (bFromSweep :type Boolean) (SweepResult :type Hit%20Result%20Structure%20%28by%20ref%29))
  (bind _glovespotlight (Variables|Default|GetGloveSpotLight))
  (Utilities|Casting|CastToBP_FirstPersonCharacter OtherActor)
  (Audio|PlaySoundatLocation "/Game/Environment/SFX/spotlight-91359.spotlight-91359" (Transformation|GetActorLocation) "0, 0, 0" 8.0 1.0 0.0 0 0 0 0)
  (Collision|SetCollisionEnabled (Variables|Default|GetSphere) "NoCollision")
  (CallFunction|TurnonLight (Variables|Default|GetSpotlight5) (Variables|Default|GetHangingLight5))
  (Utilities|FlowControl|Delay 1.0)
  (CallFunction|TurnonLight (Variables|Default|GetSpotlight4) (Variables|Default|GetHangingLight4))
  (Utilities|FlowControl|Delay 1.0)
  (CallFunction|TurnonLight (Variables|Default|GetSpotlight3) (Variables|Default|GetHangingLight3))
  (Utilities|FlowControl|Delay 1.0)
  (CallFunction|TurnonLight (Variables|Default|GetSpotlight2) (Variables|Default|GetHangingLight2))
  (Utilities|FlowControl|Delay 1.0)
  (CallFunction|TurnonLight (Variables|Default|GetSpotlight1) (Variables|Default|GetHangingLight1))
  (Utilities|FlowControl|Delay 1.0)
  (CallFunction|TurnonLight (Variables|Default|GetSpotlight) (Variables|Default|GetHangingLight))
  (Utilities|FlowControl|Delay 2.0)
  (Development|SetHiddeninGame (Variables|Default|GetSpotlights) true true)
  (Audio|PlaySoundatLocation "/Game/Environment/SFX/BZZT.BZZT" (Transformation|GetActorLocation) "0, 0, 0" 8.0 1.0 0.0 0 0 0 0)
  (Utilities|FlowControl|Delay 2.0)
  (Rendering|Components|Light|SetIntensity _glovespotlight 1e+03)
  (Audio|PlaySoundatLocation "/Game/Environment/SFX/spotlight-91359.spotlight-91359" (Transformation|GetWorldLocation _glovespotlight) "0, 0, 0" 6.0 1.0 0.0 0 0 0 0)
  (Rendering|Material|SetScalarParameterValueonMaterials (Variables|Default|GetHangingLightGloves) "Light" 1.5e+03))

(event Custom|TurnOnLight
  (params (Light :type Light%20Component%20Object%20Reference) (Mesh :type Mesh%20Component%20Object%20Reference))
  (Audio|PlaySoundatLocation "/Game/Environment/SFX/spotlight-91359.spotlight-91359" (Transformation|GetWorldLocation Light) "0, 0, 0" 6.0 1.0 0.0 0 0 0 0)
  (Rendering|Components|Light|SetIntensity Light 1e+03)
  (Rendering|Material|SetScalarParameterValueonMaterials Mesh "Light" 1e+03))

(event EventBeginPlay)

(event Collision|EventActorBeginOverlap
  (params (OtherActor :type Actor%20Object%20Reference)))

(event EventTick
  (params (DeltaSeconds :type Float%20%28single-precision%29)))

(fn ConstructionScript)