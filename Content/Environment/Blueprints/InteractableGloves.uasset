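; Interactable gloves pickup that gives the first-person player visible hands and switching ability, then sets the warehouse escape mission.
; Binds to the character's hover, unhover and interact events, filtering on itself to show or hide an icon.
; Interacting while hovered plays a sound, sets the spotlight intensity and destroys the object and plane components, leaving the actor in place.
; BeginPlay also caches an elevator reference, unused here.
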(event Custom|Hovered
  (params (HitActor :type Actor%20Object%20Reference))
  (if (== HitActor self)
    (Development|SetHiddeninGame (Variables|Default|GetIcon) false false)
    (Variables|Default|SetIsHovered true)))

(event Custom|UnHovered
  (params (HitActor :type Actor%20Object%20Reference))
  (if (== HitActor self)
    (Development|SetHiddeninGame (Variables|Default|GetIcon) true false)
    (Variables|Default|SetIsHovered false)))

(event Custom|Interacted
  (params (HitActor :type Actor%20Object%20Reference))
  (if (== HitActor self)
    (if (Variables|Default|GetIsHovered)
      (bind _asbp_first_person_character (Utilities|Casting|CastToBP_FirstPersonCharacter (Game|GetPlayerCharacter 0)))
      (Rendering|SetVisibility (Variables|/Game/FirstPerson/Blueprints/BP_FirstPersonCharacter.BP_FirstPersonCharacter_C|GetHands _asbp_first_person_character) true true)
      (Variables|/Game/FirstPerson/Blueprints/BP_FirstPersonCharacter.BP_FirstPersonCharacter_C|SetCanSwitch _asbp_first_person_character true)
      (Audio|PlaySound2D "/Game/Environment/SFX/PickUpGloves.PickUpGloves" 1.0 1.0 0.0 0 0)
      (Rendering|Components|Light|SetIntensity (Variables|Default|GetSpotLight) 3e+03)
      (Components|DestroyComponent (Variables|Default|GetInteractableObject))
      (Default|UpdateMission _asbp_first_person_character "Escape the warehouse!")
      (Components|DestroyComponent (Variables|Default|GetPlane)))))

(event EventBeginPlay
  (bind _asbp_first_person_character (Utilities|Casting|CastToBP_FirstPersonCharacter (Game|GetPlayerCharacter 0)))
  (EventDispatchers|BindEventtoInteractHover _asbp_first_person_character (delegate Custom|Hovered))
  (EventDispatchers|BindEventtoInteractUnhover _asbp_first_person_character (delegate Custom|UnHovered))
  (EventDispatchers|BindEventtoInteract _asbp_first_person_character (delegate Custom|Interacted))
  (bind _outactors (Actor|GetAllActorsOfClass "/Game/Environment/Blueprints/Elevator_BP.Elevator_BP_C"))
  (Variables|Default|SetElevatorRef (Utilities|Array|Get(acopy) _outactors 1)))

(fn ConstructionScript)