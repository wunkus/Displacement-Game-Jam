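; PipeBP is a spline-driven pipe actor that builds itself in the construction script, with no active runtime logic.
; It divides the spline by SegmentLength and adds a Y-forward cylinder spline mesh per segment, storing each in the Mesh array and zeroing its "Int" material parameter.
; StartPos and EndPos sample each segment's endpoints in local space, clamping tangents to the segment length so the cylinders follow the curve.
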(event EventBeginPlay)

(event Collision|EventActorBeginOverlap
  (params (OtherActor :type Actor%20Object%20Reference)))

(event EventTick
  (params (DeltaSeconds :type Float%20%28single-precision%29)))

(fn ConstructionScript
  (for _index (range 0 (Math|Float|Truncate (/ (Spline|GetSplineLength (Variables|Default|GetSpline)) (Variables|Default|GetSegmentLength))))
    (Variables|Default|SetIndex _index)
    (bind _returnvalue (AddComponent|AddSplineMeshComponent false))
    (Utilities|Array|Add (Variables|Default|GetMesh) _returnvalue)
    (Components|StaticMesh|SetStaticMesh _returnvalue "/Engine/EngineMeshes/Cylinder.Cylinder")
    (Rendering|Material|SetScalarParameterValueonMaterials _returnvalue "Int" 0.0)
    (SplineMesh|SetForwardAxis _returnvalue "Y" true)
    (bind (_position _tangent) (CallFunction|StartPos (Variables|Default|GetIndex)))
    (bind (_position_2 _tangent_2) (CallFunction|EndPos (Variables|Default|GetIndex)))
    (SplineMesh|SetStartandEnd _returnvalue _position _tangent _position_2 _tangent_2 true :!class /Script/Engine.SplineMeshComponent)))

(fn StartPos
  (params (Index :type Integer))
  (bind _segmentlength (Variables|Default|GetSegmentLength))
  (bind _spline (Variables|Default|GetSpline))
  (bind _returnvalue (* Index _segmentlength))
  (return (Spline|GetLocationatDistanceAlongSpline _spline _returnvalue "Local") (Math|Vector|ClampVectorSize (Spline|GetTangentatDistanceAlongSpline _spline _returnvalue "Local") 0.0 (Variables|Default|GetSegmentLength))))

(fn EndPos
  (params (Index :type Integer))
  (bind _returnvalue (+ Index 1))
  (bind _segmentlength (Variables|Default|GetSegmentLength))
  (bind _spline (Variables|Default|GetSpline))
  (bind _returnvalue_2 (* _returnvalue _segmentlength))
  (return (Spline|GetLocationatDistanceAlongSpline _spline _returnvalue_2 "Local") (Math|Vector|ClampVectorSize (Spline|GetTangentatDistanceAlongSpline _spline _returnvalue_2 "Local") 0.0 (Variables|Default|GetSegmentLength))))